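; Bubble spawner actor that creates centered rows of BP_BubbleDefault along X at its own location.
; On BeginPlay it finds BP_GridConveyor and starts a looping DeltaTime timer that calls SpawnBubbles.
; While the conveyor's SwitchSpawn is on, each call spawns evenly spaced bubbles in a loop.
; A Delay inside the loop, timed by the conveyor's SpawnDelay, feeds a FlipFlop that alternates the row count between seven and eight.
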(event `self.ReceiveBeginPlay`
  (bind _returnvalue (`GameplayStatics.GetActorOfClass` "/Game/Core/Blueprints/BubbleGridSystem/BP_GridConveyor.BP_GridConveyor_C"))
  (set `self.GridConveyor` _returnvalue)
  (`KismetSystemLibrary.K2_SetTimer` null "BubbleSpawnerTick" (`self.DeltaTime`) true))

(event `SpawnBubbles`
  (bind _numberofbubbles (`self.NumberOfBubbles`))
  (bind _gridconveyor (`self.GridConveyor`))
  (switch `name` (`/Game/Core/Blueprints/BubbleGridSystem/BP_GridConveyor.SwitchSpawn` _gridconveyor)
    (:`SpawnOn`
      (for _index (range 1 (+ _numberofbubbles 1))
        (`|SpawnActorFromClass` "/Game/Core/Blueprints/Bubbles/BP_BubbleDefault.BP_BubbleDefault_C" (`KismetMathLibrary.MakeTransform` (`KismetMathLibrary.MakeVector` (+ (* (- _index (/ (- _numberofbubbles 1) 2.0)) (`self.Bubble Spawn Distance`)) (.x (`self.K2_GetActorLocation`))) (.y (`self.K2_GetActorLocation`)) (.z (`self.K2_GetActorLocation`)))) "Undefined" "MultiplyWithRoot" null null)
        (`KismetSystemLibrary.Delay` (`/Game/Core/Blueprints/BubbleGridSystem/BP_GridConveyor.SpawnDelay` _gridconveyor))
        (`/Engine/EditorBlueprintResources/StandardMacros.FlipFlop`
          (:`A`
            (set `self.NumberOfBubbles` 7))
          (:`B`
            (set `self.NumberOfBubbles` 8)))))))

(fn `BubbleSpawnerTick`
  (`self.SpawnBubbles`))

(fn `UserConstructionScript`)