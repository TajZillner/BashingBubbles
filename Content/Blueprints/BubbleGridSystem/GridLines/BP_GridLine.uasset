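; BP_GridLine is one line of the bubble grid system, spawning and holding a row of BP_GridSquare actors.
; On BeginPlay it places a starting number of squares along its spline at a fixed spacing, offset from the spline's midpoint.
; Each square is stored in GridSpaces and attached to the line with relative transforms, using local spline positions.
; GridLineTick and the construction script are empty.
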(event `self.ReceiveBeginPlay`
  (bind _spline (`self.Spline`))
  ; SpawnRow
  (for _index (range 1 (+ (`self.GridStartingAmount`) 1))
    (bind _returnvalue (`|SpawnActorFromClass` "/Game/Blueprints/BubbleGridSystem/BP_GridSquare.BP_GridSquare_C" (`KismetMathLibrary.MakeTransform` (`SplineComponent.GetLocationAtDistanceAlongSpline` _spline (+ (* (- _index (/ (- (`self.GridStartingAmount`) 1) 2.0)) (`self.GridSpacingDistance`)) (/ (`SplineComponent.GetSplineLength` _spline) 2.0)) "Local")) "Undefined" "MultiplyWithRoot" null null))
    (`KismetArrayLibrary.Array_Add` (`self.GridSpaces`) _returnvalue)
    (`self.K2_AttachToActor` _returnvalue self "None" "KeepRelative" "KeepRelative" "KeepRelative" true)))

(fn `GridLineTick`)

(fn `UserConstructionScript`)