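; Conveyor actor for the bubble grid system that spawns rows of grid lines at a spline's start and moves them downward along it.
; A looping timer alternates even and odd row spawns at an interval of spacing over speed, set at BeginPlay, calling OnGridSpawned each time.
; A second looping timer, used instead of Tick, snaps rows to the spline, lowers their Z, and destroys them with their grid spaces at the end.
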(event `self.ReceiveBeginPlay`
  ; Begin Play
  (`KismetSystemLibrary.K2_SetTimer` null "SplineConveyor" (`self.DeltaTime`) true)
  (set `self.SpawnDelay` (/ (`self.SpawnSpacing`) (`self.ConveyorSpeed`)))
  (`KismetSystemLibrary.K2_SetTimer` null "SpawnSwitch" (`self.SpawnDelay`) true))

(event `SpawnSwitch`
  (bind _location (.location (`SplineComponent.GetTransformAtSplinePoint` (`self.Spline`) 0 "World" false)))
  ; Spawn Even and Odd Rows
  (`/Engine/EditorBlueprintResources/StandardMacros.FlipFlop`
    (:`A`
      (bind _returnvalue (`|SpawnActorFromClass` "/Game/Core/Blueprints/BubbleGridSystem/GridLines/BP_GridLine_Even.BP_GridLine_Even_C" (`KismetMathLibrary.MakeTransform` _location) "Undefined" "MultiplyWithRoot" null null))
      (`KismetArrayLibrary.Array_Add` (`self.GridLines`) _returnvalue)
      (`self.OnGridSpawned`))
    (:`B`
      (bind _returnvalue_2 (`|SpawnActorFromClass` "/Game/Core/Blueprints/BubbleGridSystem/GridLines/BP_GridLine_Odd.BP_GridLine_Odd_C" (`KismetMathLibrary.MakeTransform` _location) "Undefined" "MultiplyWithRoot" null null))
      (`KismetArrayLibrary.Array_Add` (`self.GridLines`) _returnvalue_2)
      (`self.OnGridSpawned`))))

(event `SplineConveyor`
  (bind _spline (`self.Spline`))
  ; Move Grid and Delete
  (set `self.SpawnDelay` (/ (`self.SpawnSpacing`) (`self.ConveyorSpeed`)))
  (if (`KismetArrayLibrary.Array_IsNotEmpty` (`self.GridLines`))
    (for (_array_element _array_index) (`self.GridLines`)
      (bind _returnvalue (`SplineComponent.GetDistanceAlongSplineAtLocation` _spline (`self.K2_GetActorLocation` _array_element) "World"))
      (`self.K2_SetActorLocation` _array_element (`KismetMathLibrary.MakeVector` (.x (`SplineComponent.GetLocationAtDistanceAlongSpline` _spline _returnvalue "World")) (.y (`SplineComponent.GetLocationAtDistanceAlongSpline` _spline _returnvalue "World")) (- (.z (`SplineComponent.GetLocationAtDistanceAlongSpline` _spline _returnvalue "World")) (* (`self.ConveyorSpeed`) (`self.DeltaTime`)))) false false)
      (if (>= _returnvalue (`SplineComponent.GetSplineLength` _spline))
        (for _array_element_2 (`/Game/Core/Blueprints/BubbleGridSystem/GridLines/BP_GridLine.GridSpaces` _array_element)
          (`self.K2_DestroyActor` _array_element_2))
        (`self.K2_DestroyActor` _array_element)
        (`KismetArrayLibrary.Array_Remove` (`self.GridLines`) _array_index)))))

(fn `GridConveryorTick`)

(fn `UserConstructionScript`)