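; Bubble row spawner that fills each new conveyor grid line with random red, green, blue or yellow bubbles.
; It binds to the grid conveyor's spawn event, spacing bubbles along X and alternating row size between the even and odd grid lines' counts.
; Unless fully random, chance rolls and a chain counter limit same-color runs, with optional bias from earlier colors.
; Color constraints use capped random rerolls.
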(event `self.ReceiveBeginPlay`
  ; Begin Play
  (bind _returnvalue (`GameplayStatics.GetActorOfClass` "/Game/Blueprints/BubbleGridSystem/BP_GridConveyor.BP_GridConveyor_C"))
  (set `self.GridConveyor` _returnvalue)
  (bind _returnvalue_2 (`GameplayStatics.GetActorOfClass` "/Game/Blueprints/BubbleGridSystem/GridLines/BP_GridLine_Even.BP_GridLine_Even_C"))
  (set `self.GridLineEven` _returnvalue_2)
  (bind _returnvalue_3 (`GameplayStatics.GetActorOfClass` "/Game/Blueprints/BubbleGridSystem/GridLines/BP_GridLine_Odd.BP_GridLine_Odd_C"))
  (set `self.GridLineOdd` _returnvalue_3)
  (add `/Game/Blueprints/BubbleGridSystem/BP_GridConveyor.OnGridSpawned` (`self.GridConveyor`) (delegate `SpawnBubbles`))
  (set `self.NumberOfBubbles` (`/Game/Blueprints/BubbleGridSystem/GridLines/BP_GridLine.GridStartingAmount` (`self.GridLineEven`))))

(event `SpawnBubbles`
  (bind _numberofbubbles (`self.NumberOfBubbles`))
  (bind _chainbubblespawnchance (`self.ChainBubbleSpawnChance`))
  ; Bubble Spawning Logic
  (for _index (range 1 (+ _numberofbubbles 1))
    (set `self.SpawnVector` (`KismetMathLibrary.MakeVector` (+ (* (- _index (/ (- _numberofbubbles 1) 2.0)) (`/Game/Blueprints/BubbleGridSystem/GridLines/BP_GridLine.GridSpacingDistance` (`self.GridLineEven`))) (.x (`self.K2_GetActorLocation`))) (.y (`self.K2_GetActorLocation`)) (.z (`self.K2_GetActorLocation`))))
    (`self.GetRandomBubble`)
    (if (`self.FullRandomSpawning`)
      ; Full Random Spawning
      (`|SpawnActorFromClass` (`self.Bubble`) (`KismetMathLibrary.MakeTransform` (`self.SpawnVector`)) "Undefined" "MultiplyWithRoot" null null)
      (else
        (switch `int` (`self.BubbleColorChainCount`)
          (:`0`
            ;; Check if Previous 1 bubble are the same as new bubble and cointinue chain
            (if (== (`self.Bubble`) (`self.Previous Bubble_1`))
              (if (<= (`KismetMathLibrary.RandomIntegerInRange` 0 100) (`self.SecondBubbleSpawnChance`))
                (`|SpawnActorFromClass` (`self.Bubble`) (`KismetMathLibrary.MakeTransform` (`self.SpawnVector`)) "Undefined" "MultiplyWithRoot" null null)
                (if (!= (`self.Previous Bubble_1`) (`self.Previous Bubble_2`))
                  (set `self.Previous Bubble_2` (`self.Previous Bubble_1`)))
                (set `self.Previous Bubble_1` (`self.Bubble`))
                (`/Engine/EditorBlueprintResources/StandardMacros.IncrementInt` (`self.BubbleColorChainCount`))
                (else
                  (`self.GetNewRandomBubble` :!label _label)
                  (`|SpawnActorFromClass` (`self.Bubble`) (`KismetMathLibrary.MakeTransform` (`self.SpawnVector`)) "Undefined" "MultiplyWithRoot" null null :!label _label_2)
                  (if (!= (`self.Previous Bubble_1`) (`self.Previous Bubble_2`))
                    (set `self.Previous Bubble_2` (`self.Previous Bubble_1`)))
                  (set `self.Previous Bubble_1` (`self.Bubble`))
                  (set `self.BubbleColorChainCount` 0)))
              (elif (not (`self.ChainBiasSpawning`))
                (goto _label)
                (else
                  ;; Check if Previous 2 bubble are the same as new bubble and start new chain
                  (if (== (`self.Bubble`) (`self.Previous Bubble_2`))
                    (if (not (<= (`KismetMathLibrary.RandomIntegerInRange` 0 100) _chainbubblespawnchance))
                      (goto _label)
                      (else
                        (goto _label_2)))
                    (elif (not (<= (`KismetMathLibrary.RandomIntegerInRange` 0 100) _chainbubblespawnchance))
                      (goto _label_2)
                      (else
                        (`self.GetSamePrevious2Bubble`)
                        (goto _label_2))))))))
          (:`1`
            (if (<= (`KismetMathLibrary.RandomIntegerInRange` 0 100) (`self.ThirdBubbleSpawnChance`))
              (`|SpawnActorFromClass` (`self.Bubble`) (`KismetMathLibrary.MakeTransform` (`self.SpawnVector`)) "Undefined" "MultiplyWithRoot" null null)
              (if (!= (`self.Previous Bubble_1`) (`self.Previous Bubble_2`))
                (set `self.Previous Bubble_2` (`self.Previous Bubble_1`)))
              (set `self.Previous Bubble_1` (`self.Bubble`))
              (`/Engine/EditorBlueprintResources/StandardMacros.IncrementInt` (`self.BubbleColorChainCount`))
              (else
                (`self.GetNewRandomBubble`)
                (`|SpawnActorFromClass` (`self.Bubble`) (`KismetMathLibrary.MakeTransform` (`self.SpawnVector`)) "Undefined" "MultiplyWithRoot" null null)
                (if (!= (`self.Previous Bubble_1`) (`self.Previous Bubble_2`))
                  (set `self.Previous Bubble_2` (`self.Previous Bubble_1`)))
                (set `self.Previous Bubble_1` (`self.Bubble`))
                (set `self.BubbleColorChainCount` 0))))
          (:`2`
            (`self.GetNewRandomBubble`)
            (`|SpawnActorFromClass` (`self.Bubble`) (`KismetMathLibrary.MakeTransform` (`self.SpawnVector`)) "Undefined" "MultiplyWithRoot" null null)
            (if (!= (`self.Previous Bubble_1`) (`self.Previous Bubble_2`))
              (set `self.Previous Bubble_2` (`self.Previous Bubble_1`)))
            (set `self.Previous Bubble_1` (`self.Bubble`))
            (set `self.BubbleColorChainCount` 0))))))
  (`/Engine/EditorBlueprintResources/StandardMacros.FlipFlop`
    (:`A`
      (set `self.NumberOfBubbles` (`/Game/Blueprints/BubbleGridSystem/GridLines/BP_GridLine.GridStartingAmount` (`self.GridLineOdd`))))
    (:`B`
      (set `self.NumberOfBubbles` (`/Game/Blueprints/BubbleGridSystem/GridLines/BP_GridLine.GridStartingAmount` (`self.GridLineEven`))))))

(fn `BubbleSpawnerTick`
  (`self.SpawnBubbles`))

(fn `GetNewRandomBubble`
  (for _ (range 41)
    (switch `int` (`KismetMathLibrary.RandomIntegerInRange` 1 4)
      (:`1`
        (set `self.Bubble` "/Game/Blueprints/Bubbles/BP_RedBubble.BP_RedBubble_C"))
      (:`2`
        (set `self.Bubble` "/Game/Blueprints/Bubbles/BP_GreenBubble.BP_GreenBubble_C"))
      (:`3`
        (set `self.Bubble` "/Game/Blueprints/Bubbles/BP_BlueBubble.BP_BlueBubble_C"))
      (:`4`
        (set `self.Bubble` "/Game/Blueprints/Bubbles/BP_YellowBubble.BP_YellowBubble_C")))
    (if (!= (`self.Bubble`) (`self.Previous Bubble_1`))
      (break)))
  (return))

(fn `GetRandomBubble`
  (switch `int` (`KismetMathLibrary.RandomIntegerInRange` 1 4)
    (:`1`
      (set `self.Bubble` "/Game/Blueprints/Bubbles/BP_RedBubble.BP_RedBubble_C"))
    (:`2`
      (set `self.Bubble` "/Game/Blueprints/Bubbles/BP_GreenBubble.BP_GreenBubble_C"))
    (:`3`
      (set `self.Bubble` "/Game/Blueprints/Bubbles/BP_BlueBubble.BP_BlueBubble_C"))
    (:`4`
      (set `self.Bubble` "/Game/Blueprints/Bubbles/BP_YellowBubble.BP_YellowBubble_C"))))

(fn `GetSamePrevious2Bubble`
  (for _ (range 41)
    (switch `int` (`KismetMathLibrary.RandomIntegerInRange` 1 4)
      (:`1`
        (set `self.Bubble` "/Game/Blueprints/Bubbles/BP_RedBubble.BP_RedBubble_C"))
      (:`2`
        (set `self.Bubble` "/Game/Blueprints/Bubbles/BP_GreenBubble.BP_GreenBubble_C"))
      (:`3`
        (set `self.Bubble` "/Game/Blueprints/Bubbles/BP_BlueBubble.BP_BlueBubble_C"))
      (:`4`
        (set `self.Bubble` "/Game/Blueprints/Bubbles/BP_YellowBubble.BP_YellowBubble_C")))
    (if (== (`self.Bubble`) (`self.Previous Bubble_2`))
      (break))))

(fn `UserConstructionScript`)