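; BP_BubbleSpawner spawns rows of randomly colored bubbles for the grid conveyor.
; On BeginPlay it caches the conveyor and both grid line actors, then binds SpawnBubbles to the conveyor's grid-spawned event.
; Each spawn lays bubbles along X using the even line's spacing, then a FlipFlop alternates the next row's count between odd and even lines.
; BubbleSpawnerTick also exposes a direct spawn call.
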(event `self.ReceiveBeginPlay`
  ; Begin Play
  (bind _returnvalue (`GameplayStatics.GetActorOfClass` "/Game/Core/Blueprints/BubbleGridSystem/BP_GridConveyor.BP_GridConveyor_C"))
  (set `self.GridConveyor` _returnvalue)
  (bind _returnvalue_2 (`GameplayStatics.GetActorOfClass` "/Game/Core/Blueprints/BubbleGridSystem/GridLines/BP_GridLine_Even.BP_GridLine_Even_C"))
  (set `self.GridLineEven` _returnvalue_2)
  (bind _returnvalue_3 (`GameplayStatics.GetActorOfClass` "/Game/Core/Blueprints/BubbleGridSystem/GridLines/BP_GridLine_Odd.BP_GridLine_Odd_C"))
  (set `self.GridLineOdd` _returnvalue_3)
  (add `/Game/Core/Blueprints/BubbleGridSystem/BP_GridConveyor.OnGridSpawned` (`self.GridConveyor`) (delegate `SpawnBubbles`))
  (set `self.NumberOfBubbles` (`/Game/Core/Blueprints/BubbleGridSystem/GridLines/BP_GridLine.GridStartingAmount` (`self.GridLineEven`))))

(event `SpawnBubbles`
  (bind _numberofbubbles (`self.NumberOfBubbles`))
  (for _index (range 1 (+ _numberofbubbles 1))
    (bind _output_get (set `self.SpawnVector` (`KismetMathLibrary.MakeVector` (+ (* (- _index (/ (- _numberofbubbles 1) 2.0)) (`/Game/Core/Blueprints/BubbleGridSystem/GridLines/BP_GridLine.GridSpacingDistance` (`self.GridLineEven`))) (.x (`self.K2_GetActorLocation`))) (.y (`self.K2_GetActorLocation`)) (.z (`self.K2_GetActorLocation`)))))
    (switch `int` (`KismetMathLibrary.RandomIntegerInRange` 1 4)
      (:`1`
        (set `self.Bubble` "/Game/Core/Blueprints/Bubbles/BP_RedBubble.BP_RedBubble_C"))
      (:`2`
        (set `self.Bubble` "/Game/Core/Blueprints/Bubbles/BP_GreenBubble.BP_GreenBubble_C"))
      (:`3`
        (set `self.Bubble` "/Game/Core/Blueprints/Bubbles/BP_BlueBubble.BP_BlueBubble_C"))
      (:`4`
        (set `self.Bubble` "/Game/Core/Blueprints/Bubbles/BP_YellowBubble.BP_YellowBubble_C")))
    (`|SpawnActorFromClass` (`self.Bubble`) (`KismetMathLibrary.MakeTransform` _output_get) "Undefined" "MultiplyWithRoot" null null))
  (`/Engine/EditorBlueprintResources/StandardMacros.FlipFlop`
    (:`A`
      (set `self.NumberOfBubbles` (`/Game/Core/Blueprints/BubbleGridSystem/GridLines/BP_GridLine.GridStartingAmount` (`self.GridLineOdd`))))
    (:`B`
      (set `self.NumberOfBubbles` (`/Game/Core/Blueprints/BubbleGridSystem/GridLines/BP_GridLine.GridStartingAmount` (`self.GridLineEven`))))))

(fn `BubbleSpawnerTick`
  (`self.SpawnBubbles`))

(fn `UserConstructionScript`)