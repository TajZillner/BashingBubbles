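; Default bubble actor for a colour-matching bubble game, tracking same-colour chains through BP_GameInstance.
; Overlaps with actors tagged in its colour grow the shared chain and active count, with a once-only decrement that resets on the NotPopped event.
; KillBubble adds score and destroys it; debug keys toggle interaction collision or play a two-phase detach, hop and fall before destruction.
; BubblePop, the construction script and CheckAttatchedBellow are unfinished stubs.
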(event OnComponentBeginOverlap(BubbleInteractionCollision)
  (params (OverlappedComponent :type Primitive%20Component%20Object%20Reference) (OtherActor :type Actor%20Object%20Reference) (OtherComp :type Primitive%20Component%20Object%20Reference) (OtherBodyIndex :type Integer) (bFromSweep :type Boolean) (SweepResult :type Hit%20Result%20Structure%20%28by%20ref%29))
  (bind _gameinstance (Variables|Default|GetGameInstance))
  (bind _bubblechain (Variables|/Game/Core/BP_GameInstance.BP_GameInstance_C|GetBubbleChain _gameinstance))
  (bind _activebubbles (Variables|/Game/Core/BP_GameInstance.BP_GameInstance_C|GetActiveBubbles _gameinstance))
  ;[0.15 0.15 0.15 0.5] Bubble On Bubble Collision Logic
  (if (Actor|ActorHasTag OtherActor (Utilities|Struct|BreakS_BubbleStats (Variables|Default|GetBubbleStats)))
    (if (not (Variables|Default|GetBubbleTriggered))
      (Variables|Default|SetBubbleTriggered true)
      (if (not (Utilities|Array|ContainsItem _bubblechain OtherActor))
        (Utilities|Array|Add _bubblechain OtherActor)
        (Math|Integer|IncrementInt (Variables|/Game/Core/BP_GameInstance.BP_GameInstance_C|GetBubbleChainCount _gameinstance)
          (:%20%20
            (Math|Integer|IncrementInt _activebubbles))))
      (else
        (Utilities|FlowControl|DoOnce false
          (:Completed
            (Math|Integer|DecrementInt _activebubbles)))))))

(event Custom|NotPopped
  ;[0.15 0.15 0.15 0.5] Bubble On Bubble Collision Logic
  (Variables|Default|SetBubbleTriggered false)
  (Utilities|FlowControl|DoOnce false) ; enters at Reset
)

(event Custom|KillBubble
  (bind _gameinstance (Variables|Default|GetGameInstance))
  ;[0.15 0.15 0.15 0.5] Generic Kill Bubble Function
  (Variables|/Game/Core/BP_GameInstance.BP_GameInstance_C|SetTotal%20Score _gameinstance (+ (Variables|/Game/Core/BP_GameInstance.BP_GameInstance_C|GetTotal%20Score _gameinstance) 100))
  (Actor|DestroyActor))

(event Custom|BubblePop
  ;[0.15 0.15 0.15 0.5] BubbleFallingAnimation
)

(event EventBeginPlay
  ;[0.15 0.15 0.15 0.5] BeginPlay
  (bind _asbp_game_instance (Utilities|Casting|CastToBP_GameInstance (Game|GetGameInstance)))
  (bind _output_get (Variables|Default|SetGameInstance _asbp_game_instance))
  (EventDispatchers|BindEventtoOnNotPopped _output_get (delegate Custom|NotPopped)))

(event Input|KeyboardEvents|DebugKey1
  (params (Key :type Key%20Structure :default "None") (ActionValue :type Input%20Action%20Value%20Structure))
  (bind _bubbleinteractioncollision (Variables|Default|GetBubbleInteractionCollision))
  (:Pressed
    (Collision|SetCollisionEnabled _bubbleinteractioncollision "QueryOnly"))
  (:Released
    (Collision|SetCollisionEnabled _bubbleinteractioncollision "NoCollision")))

(event Input|KeyboardEvents|DebugKey2
  (params (Key :type Key%20Structure :default "None") (ActionValue :type Input%20Action%20Value%20Structure))
  (bind _returnvalue (Transformation|GetActorLocation))
  (bind _tags (Variables|Actor|GetTags))
  (bind _animationswitch (Variables|Default|GetAnimationSwitch))
  ;[0.15 0.15 0.15 0.5] BubbleFallingAnimation
  (:Pressed
    (Utilities|Array|SetArrayElem _tags (Utilities|Array|FindItem _tags "OnGrid") "OffGrid")
    (Transformation|DetachFromActor "KeepWorld" "KeepWorld" "KeepWorld")
    (bind _alpha (Timeline|FallingAnimation Play)
      (:Update
        (switch int (Variables|Default|GetAnimationSwitch)
          (:0
            (Transformation|SetActorRelativeLocation (Math|Interpolation|Ease "Linear" _alpha _returnvalue (+ _returnvalue "0.000000,0.000000,2.500000"))))
          (:1
            (Transformation|SetActorRelativeLocation (Math|Interpolation|Ease "Linear" _alpha _returnvalue (+ _returnvalue "0.000000,0.000000,-1.250000"))))))
      (:Finished
        (switch int _animationswitch
          (:0
            (Math|Integer|IncrementInt _animationswitch
              (:%20%20
                (Timeline|FallingAnimation PlayFromStart))))
          (:1
            (Actor|DestroyActor)))))))

(fn ConstructionScript)

(fn CheckAttatchedBellow)